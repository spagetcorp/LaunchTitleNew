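; WreckedKitchenVent is a vent trigger that sends the player to WreckedKitchenLevel once they have found the screwdriver.
; On box overlap it checks ScrewDriverFound on the PlayerCharacter; if set, it shows a Fading widget, disables input and opens the level after a short delay.
; Without the screwdriver it only shows a second Fading widget, which is removed when the player leaves the box.
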(event OnComponentBeginOverlap(Box)
  (params (OverlappedComponent :type Primitive%20Component%20Object%20Reference) (OtherActor :type Actor%20Object%20Reference) (OtherComp :type Primitive%20Component%20Object%20Reference) (OtherBodyIndex :type Integer) (bFromSweep :type Boolean) (SweepResult :type Hit%20Result%20Structure%20%28by%20ref%29))
  (bind _asplayer_character (Utilities|Casting|CastToPlayerCharacter OtherActor))
  (if (Variables|/Game/Blueprints/PlayerCharacter.PlayerCharacter_C|GetScrewDriverFound _asplayer_character)
    (bind _returnvalue (UserInterface|CreateWidget "/Game/Blueprints/Fading.Fading_C"))
    (UserInterface|Viewport|AddtoViewport _returnvalue 0)
    (Input|DisableInput _asplayer_character 0)
    (Utilities|FlowControl|Delay 1.5)
    (Game|OpenLevel(byName) "WreckedKitchenLevel")
    (else
      (bind _returnvalue_2 (UserInterface|CreateWidget "/Game/Blueprints/Fading.Fading_C"))
      (UserInterface|Viewport|AddtoViewport _returnvalue_2 0))))

(event OnComponentEndOverlap(Box)
  (params (OverlappedComponent :type Primitive%20Component%20Object%20Reference) (OtherActor :type Actor%20Object%20Reference) (OtherComp :type Primitive%20Component%20Object%20Reference) (OtherBodyIndex :type Integer))
  (Utilities|Casting|CastToPlayerCharacter OtherActor)
  (Widget|RemovefromParent (stale OnComponentBeginOverlap(Box) _returnvalue_2)))

(fn ConstructionScript)