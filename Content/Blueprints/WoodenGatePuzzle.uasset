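; Wooden gate puzzle actor that opens once a player holding the gate key overlaps its trigger box.
; The overlap checks GateKeyFound on PlayerCharacter, plays a lock click at the world origin and sets the player's GateOverlapped flag.
; After a short delay, a timeline drives a rotation lerp on StaticMesh1 from StartPos to EndPos to swing the gate.
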(event OnComponentBeginOverlap(Box)
  (params (OverlappedComponent :type Primitive%20Component%20Object%20Reference) (OtherActor :type Actor%20Object%20Reference) (OtherComp :type Primitive%20Component%20Object%20Reference) (OtherBodyIndex :type Integer) (bFromSweep :type Boolean) (SweepResult :type Hit%20Result%20Structure%20%28by%20ref%29))
  (bind _asplayer_character (Utilities|Casting|CastToPlayerCharacter OtherActor))
  (if (Variables|/Game/Blueprints/PlayerCharacter.PlayerCharacter_C|GetGateKeyFound? _asplayer_character)
    (Audio|PlaySoundatLocation "/Game/Sounds/GateLockClick.GateLockClick" "0, 0, 0" "0, 0, 0" 1.0 1.0 0.0 0 0 0)
    (Variables|/Game/Blueprints/PlayerCharacter.PlayerCharacter_C|SetGateOverlapped _asplayer_character true)
    (Utilities|FlowControl|Delay 1.5)
    (bind _newtrack_0 (Timeline|Timeline_0 Play)
      (:Update
        (Transformation|SetRelativeRotation (Variables|Default|GetStaticMesh1) (Math|Rotator|Lerp(Rotator) (Variables|Default|GetStartPos) (Variables|Default|GetEndPos) _newtrack_0) false false)))))

(fn ConstructionScript)