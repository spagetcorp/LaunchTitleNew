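; ExitWindow is a camera-angle trigger volume that changes the player's camera while the PlayerCharacter is inside its Box.
; On begin overlap, it offsets the character's Camera sideways along local Y and sets a tilted or turned world rotation on the ActiveCamera actor.
; On end overlap, it zeroes the Camera's relative location and the ActiveCamera's relative rotation.
; Both changes snap instantly, with no interpolation or blending.
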(event OnComponentBeginOverlap(Box)
  (params (OverlappedComponent :type Primitive%20Component%20Object%20Reference) (OtherActor :type Actor%20Object%20Reference) (OtherComp :type Primitive%20Component%20Object%20Reference) (OtherBodyIndex :type Integer) (bFromSweep :type Boolean) (SweepResult :type Hit%20Result%20Structure%20%28by%20ref%29))
  (bind _asplayer_character (Utilities|Casting|CastToPlayerCharacter OtherActor))
  (Transformation|SetRelativeLocation (Variables|/Game/Blueprints/PlayerCharacter.PlayerCharacter_C|GetCamera _asplayer_character) "0.000000,-500.000000,0.000000" false false)
  (Transformation|SetActorRotation (Variables|/Game/Blueprints/PlayerCharacter.PlayerCharacter_C|GetActiveCamera _asplayer_character) "0.000000,25.000000,0.000000"))

(event OnComponentEndOverlap(Box)
  (params (OverlappedComponent :type Primitive%20Component%20Object%20Reference) (OtherActor :type Actor%20Object%20Reference) (OtherComp :type Primitive%20Component%20Object%20Reference) (OtherBodyIndex :type Integer))
  (bind _asplayer_character (Utilities|Casting|CastToPlayerCharacter OtherActor))
  (Transformation|SetRelativeLocation (Variables|/Game/Blueprints/PlayerCharacter.PlayerCharacter_C|GetCamera _asplayer_character) "0, 0, 0" false false)
  (Transformation|SetActorRelativeRotation (Variables|/Game/Blueprints/PlayerCharacter.PlayerCharacter_C|GetActiveCamera _asplayer_character)))

(fn ConstructionScript)