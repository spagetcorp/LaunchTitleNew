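; EscapeWindow is an actor for a window that opens when a player who has found the window key enters its trigger box.
; The box overlap casts to PlayerCharacter and checks WindowKeyFound, then plays a gate lock click at the world origin.
; After a short delay, a timeline lerps StaticMesh1's relative location between two stored positions to slide it.
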(event OnComponentBeginOverlap(Box)
  (params (OverlappedComponent :type Primitive%20Component%20Object%20Reference) (OtherActor :type Actor%20Object%20Reference) (OtherComp :type Primitive%20Component%20Object%20Reference) (OtherBodyIndex :type Integer) (bFromSweep :type Boolean) (SweepResult :type Hit%20Result%20Structure%20%28by%20ref%29))
  (bind _asplayer_character (Utilities|Casting|CastToPlayerCharacter OtherActor))
  (if (Variables|/Game/Blueprints/PlayerCharacter.PlayerCharacter_C|GetWindowKeyFound? _asplayer_character)
    (Audio|PlaySoundatLocation "/Game/Sounds/GateLockClick.GateLockClick" "0, 0, 0" "0, 0, 0" 1.0 1.0 0.0 0 0 0)
    (Utilities|FlowControl|Delay 0.5)
    (bind _newtrack_0 (Timeline|Timeline_0 Play)
      (:Update
        (Transformation|SetRelativeLocation (Variables|Default|GetStaticMesh1) (Math|Vector|Lerp(Vector) (Variables|Default|GetLocation%201) (Variables|Default|GetLocation%202) _newtrack_0) false false)))))

(fn ConstructionScript)