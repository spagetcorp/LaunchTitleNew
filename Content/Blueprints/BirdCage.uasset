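; Bird cage the player knocks along in stages until it falls and sets BirdCageFallen on PlayerCharacter.
; Entering ReadyBox arms it, and each player overlap with HitBox consumes that to advance one stage, tracked by CageHit booleans.
; Timelines lerp the cage between set locations with dragging sounds.
; The fourth hit chains into a move and rotation, then a wood scrape and Pivot rotation.
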(event OnComponentBeginOverlap(HitBox)
  (params (OverlappedComponent :type Primitive%20Component%20Object%20Reference) (OtherActor :type Actor%20Object%20Reference) (OtherComp :type Primitive%20Component%20Object%20Reference) (OtherBodyIndex :type Integer) (bFromSweep :type Boolean) (SweepResult :type Hit%20Result%20Structure%20%28by%20ref%29))
  (bind _birdcage (Variables|Default|GetBirdCage))
  (if (Variables|Default|GetReady)
    (Utilities|Casting|CastToPlayerCharacter OtherActor)
    (Variables|Default|SetReady false)
    (if (Variables|Default|GetCageHit0)
      (bind _newtrack_0 (Timeline|Cage%20Move Play)
        (:Update
          (Transformation|SetRelativeLocation (Variables|Default|GetBirdCage) (Math|Vector|Lerp(Vector) (Variables|Default|GetLocation%201) (Variables|Default|GetLocation%202) _newtrack_0) false false)
          (Variables|Default|SetCageHit1 true)
          (Variables|Default|SetCageHit0 false)
          (Utilities|FlowControl|DoOnce false
            (:Completed
              (Audio|PlaySoundatLocation "/Game/Sounds/Dragging.Dragging" "0, 0, 0" "0, 0, 0" 1.0 1.0 0.0 0 0 0)))))
      (elif (Variables|Default|GetCageHit1)
        (bind _newtrack_0_2 (Timeline|Timeline_0 Play)
          (:Update
            (Transformation|SetRelativeLocation (Variables|Default|GetBirdCage) (Math|Vector|Lerp(Vector) (Variables|Default|GetLocation%202) (Variables|Default|GetLocation%203) _newtrack_0_2) false false)
            (Variables|Default|SetCageHit2 true)
            (Variables|Default|SetCageHit1 false)
            (Utilities|FlowControl|DoOnce false
              (:Completed
                (Audio|PlaySoundatLocation "/Game/Sounds/Dragging.Dragging" "0, 0, 0" "0, 0, 0" 1.0 1.0 0.0 0 0 0)))))
        (elif (Variables|Default|GetCageHit2)
          (bind _newtrack_0_3 (Timeline|Timeline_1 Play)
            (:Update
              (Transformation|SetRelativeLocation (Variables|Default|GetBirdCage) (Math|Vector|Lerp(Vector) (Variables|Default|GetLocation%203) (Variables|Default|GetLocation%204) _newtrack_0_3) false false)
              (Variables|Default|SetCageHit3 true)
              (Variables|Default|SetCageHit2 false)
              (Utilities|FlowControl|DoOnce false
                (:Completed
                  (Audio|PlaySoundatLocation "/Game/Sounds/Dragging.Dragging" "0, 0, 0" "0, 0, 0" 1.0 1.0 0.0 0 0 0)))))
          (elif (Variables|Default|GetCageHit3)
            (bind _newtrack_0_4 (Timeline|Timeline_2 Play)
              (:Update
                (Transformation|SetRelativeLocation (Variables|Default|GetBirdCage) (Math|Vector|Lerp(Vector) (Variables|Default|GetLocation%204) (Variables|Default|GetLocation%205) _newtrack_0_4) false false)
                (Utilities|FlowControl|DoOnce false
                  (:Completed
                    (Audio|PlaySoundatLocation "/Game/Sounds/Dragging.Dragging" "0, 0, 0" "0, 0, 0" 1.0 1.0 0.0 0 0 0)
                    (Utilities|FlowControl|Delay 0.1)
                    (bind _newtrack_0_5 (Timeline|Timeline_3 Play)
                      (:Update
                        (Transformation|SetRelativeLocation _birdcage (Math|Vector|Lerp(Vector) (Variables|Default|GetLocation%205) (Variables|Default|GetLocation%206) _newtrack_0_5) false false)
                        (bind _newtrack_0_6 (Timeline|Timeline_4 Play)
                          (:Update
                            (Transformation|SetRelativeRotation _birdcage (Math|Rotator|Lerp(Rotator) (Variables|Default|GetStartPos) (Variables|Default|GetEndPos) _newtrack_0_6) false false)
                            (Variables|Default|SetCageHit3 false))
                          (:Finished
                            (Utilities|FlowControl|DoOnce false
                              (:Completed
                                (Audio|PlaySoundatLocation "/Game/Sounds/StudentSounds/Nicole/woodscrape.woodscrape" "0, 0, 0" "0, 0, 0" 1.0 1.0 0.0 0 0 0)
                                (bind _newtrack_0_7 (Timeline|Timeline_5 Play)
                                  (:Update
                                    (Transformation|SetRelativeRotation (Variables|Default|GetPivot) (Math|Rotator|Lerp(Rotator) (Variables|Default|GetStartPos) (Variables|Default|GetEndPos2) _newtrack_0_7) false false)
                                    (bind _asplayer_character (Utilities|Casting|CastToPlayerCharacter (Game|GetPlayerCharacter 0)))
                                    (Variables|/Game/Blueprints/PlayerCharacter.PlayerCharacter_C|SetBirdCageFallen _asplayer_character true)))))))))))))))))))

(event OnComponentBeginOverlap(ReadyBox)
  (params (OverlappedComponent :type Primitive%20Component%20Object%20Reference) (OtherActor :type Actor%20Object%20Reference) (OtherComp :type Primitive%20Component%20Object%20Reference) (OtherBodyIndex :type Integer) (bFromSweep :type Boolean) (SweepResult :type Hit%20Result%20Structure%20%28by%20ref%29))
  (Utilities|Casting|CastToPlayerCharacter OtherActor)
  (Variables|Default|SetReady true))

(event OnComponentEndOverlap(ReadyBox)
  (params (OverlappedComponent :type Primitive%20Component%20Object%20Reference) (OtherActor :type Actor%20Object%20Reference) (OtherComp :type Primitive%20Component%20Object%20Reference) (OtherBodyIndex :type Integer))
  (Utilities|Casting|CastToPlayerCharacter OtherActor)
  (Utilities|FlowControl|Delay 0.5)
  (Variables|Default|SetReady false))

(fn ConstructionScript)