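; RaftersPlank1 is a shootable rafter plank whose two halves, Cube and Cube1, animate when a ShotgunBullet overlaps its Box.
; Each half rolls on its own timeline, then after a short delay a second timeline drives its height, with the halves held at opposite Y offsets.
; All motion uses relative transforms from timeline curves rather than physics, and no guard blocks later hits from retriggering it.
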(event OnComponentBeginOverlap(Box)
  (params (OverlappedComponent :type Primitive%20Component%20Object%20Reference) (OtherActor :type Actor%20Object%20Reference) (OtherComp :type Primitive%20Component%20Object%20Reference) (OtherBodyIndex :type Integer) (bFromSweep :type Boolean) (SweepResult :type Hit%20Result%20Structure%20%28by%20ref%29))
  (Utilities|Casting|CastToShotgunBullet OtherActor)
  (Utilities|FlowControl|Sequence
    (:then_0
      (bind _newtrack_2 (Timeline|Timeline_0 Play)
        (:Update
          (Transformation|SetRelativeRotation (Variables|Default|GetCube) (Math|Rotator|MakeRotator _newtrack_2 0.0 0.0) false false))))
    (:then_1
      (Utilities|FlowControl|Delay 0.4)
      (bind _newtrack_0 (Timeline|Timeline_1 Play)
        (:Update
          (Transformation|SetRelativeLocation (Variables|Default|GetCube) (Math|Vector|MakeVector 0.0 2.5e+02 _newtrack_0) false false))))
    (:then_2
      (bind _newtrack_0_2 (Timeline|Timeline_2 Play)
        (:Update
          (Transformation|SetRelativeRotation (Variables|Default|GetCube1) (Math|Rotator|MakeRotator _newtrack_0_2 0.0 0.0) false false))))
    (:then_3
      (Utilities|FlowControl|Delay 0.4)
      (bind _newtrack_0_3 (Timeline|Timeline_3 Play)
        (:Update
          (Transformation|SetRelativeLocation (Variables|Default|GetCube1) (Math|Vector|MakeVector 0.0 -2.5e+02 _newtrack_0_3) false false))))))

(fn ConstructionScript)