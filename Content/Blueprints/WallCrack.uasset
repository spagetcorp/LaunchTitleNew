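; WallCrack is a trigger actor that teleports the player to a hard-coded location once the PlayerCharacter's PaintingFallen flag is set.
; Its Box overlap checks that flag, waits briefly, then shows a FadingFast widget to cover the transition.
; It calls DisableInput and EnableInput on itself around a short delay, with no controller specified, then teleports the character and removes the widget.
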(event OnComponentBeginOverlap(Box)
  (params (OverlappedComponent :type Primitive%20Component%20Object%20Reference) (OtherActor :type Actor%20Object%20Reference) (OtherComp :type Primitive%20Component%20Object%20Reference) (OtherBodyIndex :type Integer) (bFromSweep :type Boolean) (SweepResult :type Hit%20Result%20Structure%20%28by%20ref%29))
  (bind _asplayer_character (Utilities|Casting|CastToPlayerCharacter OtherActor))
  (if (Variables|/Game/Blueprints/PlayerCharacter.PlayerCharacter_C|GetPaintingFallen _asplayer_character)
    (Utilities|FlowControl|Delay 0.2)
    (bind _returnvalue (UserInterface|CreateWidget "/Game/Blueprints/FadingFast.FadingFast_C"))
    (UserInterface|Viewport|AddtoViewport _returnvalue 0)
    (Input|DisableInput 0)
    (Utilities|FlowControl|Delay 0.5)
    (Input|EnableInput 0)
    (Transformation|Teleport _asplayer_character "1086.772095,-63445.292969,1330.000000" "0,90.000000, 0")
    (Widget|RemovefromParent _returnvalue)))

(event EventBeginPlay)

(event Collision|EventActorBeginOverlap
  (params (OtherActor :type Actor%20Object%20Reference)))

(event EventTick
  (params (DeltaSeconds :type Float%20%28single-precision%29)))

(fn ConstructionScript)