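; Chest is an interactable chest that opens when a player who has found the chest key overlaps its Box trigger.
; With the key, it flags ChestOpened on the PlayerCharacter, then once only plays a lock click sound and runs a timeline that rotates the Pivot between start and end rotations.
; Without the key, it briefly raises the player's ChestKeyNeeded flag, then clears it after a short delay.
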(event OnComponentBeginOverlap(Box)
  (params (OverlappedComponent :type Primitive%20Component%20Object%20Reference) (OtherActor :type Actor%20Object%20Reference) (OtherComp :type Primitive%20Component%20Object%20Reference) (OtherBodyIndex :type Integer) (bFromSweep :type Boolean) (SweepResult :type Hit%20Result%20Structure%20%28by%20ref%29))
  (bind _asplayer_character (Utilities|Casting|CastToPlayerCharacter OtherActor))
  (if (Variables|/Game/Blueprints/PlayerCharacter.PlayerCharacter_C|GetChestKeyFound? _asplayer_character)
    (Variables|/Game/Blueprints/PlayerCharacter.PlayerCharacter_C|SetChestOpened _asplayer_character true)
    (Utilities|FlowControl|DoOnce false
      (:Completed
        (Audio|PlaySoundatLocation "/Game/Sounds/GateLockClick.GateLockClick" "0, 0, 0" "0, 0, 0" 1.0 1.0 0.0 0 0 0)
        (bind _newtrack_0 (Timeline|Timeline_0 Play)
          (:Update
            (Transformation|SetRelativeRotation (Variables|Default|GetPivot) (Math|Rotator|Lerp(Rotator) (Variables|Default|GetStartPos) (Variables|Default|GetEndPos) _newtrack_0) false false)))))
    (else
      (Variables|/Game/Blueprints/PlayerCharacter.PlayerCharacter_C|SetChestKeyNeeded _asplayer_character true)
      (Utilities|FlowControl|Delay 0.2)
      (Variables|/Game/Blueprints/PlayerCharacter.PlayerCharacter_C|SetChestKeyNeeded _asplayer_character false))))

(event EventBeginPlay)

(event Collision|EventActorBeginOverlap
  (params (OtherActor :type Actor%20Object%20Reference)))

(event EventTick
  (params (DeltaSeconds :type Float%20%28single-precision%29)))

(fn ConstructionScript)