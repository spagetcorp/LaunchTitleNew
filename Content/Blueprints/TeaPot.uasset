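; TeaPot is a one-shot scripted event that drags and topples a teapot, represented by Cylinder, when the player enters its Box trigger.
; The overlap sets TeaPotCamera on PlayerCharacter, destroys the trigger and starts chained timelines that lerp Cylinder's location and rotation.
; DoOnce gates play the dragging sound as movement starts and, once rotation finishes, the crash sound before setting the player's TeaPotFall flag.
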(event OnComponentBeginOverlap(Box)
  (params (OverlappedComponent :type Primitive%20Component%20Object%20Reference) (OtherActor :type Actor%20Object%20Reference) (OtherComp :type Primitive%20Component%20Object%20Reference) (OtherBodyIndex :type Integer) (bFromSweep :type Boolean) (SweepResult :type Hit%20Result%20Structure%20%28by%20ref%29))
  (bind _cylinder (Variables|Default|GetCylinder))
  (bind _asplayer_character (Utilities|Casting|CastToPlayerCharacter OtherActor))
  (Variables|/Game/Blueprints/PlayerCharacter.PlayerCharacter_C|SetTeaPotCamera _asplayer_character true)
  (Components|DestroyComponent (Variables|Default|GetBox))
  (bind _newtrack_0 (Timeline|Timeline_0 Play)
    (:Update
      (Transformation|SetRelativeLocation (Variables|Default|GetCylinder) (Math|Vector|Lerp(Vector) (Variables|Default|GetLocation%201) (Variables|Default|GetLocation%202) _newtrack_0) false false)
      (Utilities|FlowControl|DoOnce false
        (:Completed
          (Audio|PlaySoundatLocation "/Game/Sounds/Dragging.Dragging" "0, 0, 0" "0, 0, 0" 1.0 1.0 0.0 0 0 0)
          (Utilities|FlowControl|Delay 0.1)
          (bind _newtrack_0_2 (Timeline|Timeline_1 Play)
            (:Update
              (Transformation|SetRelativeLocation _cylinder (Math|Vector|Lerp(Vector) (Variables|Default|GetLocation%202) (Variables|Default|GetLocation%203) _newtrack_0_2) false false)
              (bind _newtrack_0_3 (Timeline|Timeline_2 Play)
                (:Update
                  (Transformation|SetRelativeRotation _cylinder (Math|Rotator|Lerp(Rotator) (Variables|Default|GetStartPos) (Variables|Default|GetEndPos) _newtrack_0_3) false false))
                (:Finished
                  (Utilities|FlowControl|DoOnce false
                    (:Completed
                      (Audio|PlaySoundatLocation "/Game/Sounds/Crashing.Crashing" "0, 0, 0" "0, 0, 0" 1.0 1.0 0.0 0 0 0)
                      (Variables|/Game/Blueprints/PlayerCharacter.PlayerCharacter_C|SetTeaPotFall _asplayer_character true))))))))))))

(fn ConstructionScript)