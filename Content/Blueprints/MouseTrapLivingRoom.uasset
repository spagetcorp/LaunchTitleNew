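; Living room mouse trap that snaps shut when the player character or a pushable book overlaps its box.
; Each trigger fires once, playing the trap sound and a timeline that lerps the Pivot's rotation between StartPos and EndPos.
; For the player, timeline updates add Fading widgets, call DisableInput and open LivingRoomLevel after a delay.
; A book disarms the trap by destroying the box.
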(event OnComponentBeginOverlap(Box)
  (params (OverlappedComponent :type Primitive%20Component%20Object%20Reference) (OtherActor :type Actor%20Object%20Reference) (OtherComp :type Primitive%20Component%20Object%20Reference) (OtherBodyIndex :type Integer) (bFromSweep :type Boolean) (SweepResult :type Hit%20Result%20Structure%20%28by%20ref%29))
  (Utilities|FlowControl|Sequence
    (:then_0
      (Utilities|Casting|CastToPlayerCharacter OtherActor)
      (Utilities|FlowControl|DoOnce false
        (:Completed
          (Audio|PlaySoundatLocation "/Game/Sounds/MouseTrap.MouseTrap" "0, 0, 0" "0, 0, 0" 1.0 1.0 0.0 0 0 0)
          (bind _newtrack_0 (Timeline|Timeline_0 Play)
            (:Update
              (Transformation|SetRelativeRotation (Variables|Default|GetPivot) (Math|Rotator|Lerp(Rotator) (Variables|Default|GetStartPos) (Variables|Default|GetEndPos) _newtrack_0) false false)
              (bind _returnvalue (UserInterface|CreateWidget "/Game/Blueprints/Fading.Fading_C"))
              (UserInterface|Viewport|AddtoViewport _returnvalue 0)
              (Input|DisableInput 0)
              (Utilities|FlowControl|Delay 1.5)
              (Game|OpenLevel(byName) "LivingRoomLevel"))))))
    (:then_1
      (Utilities|Casting|CastToPushableBook OtherActor)
      (Utilities|FlowControl|DoOnce false
        (:Completed
          (Audio|PlaySoundatLocation "/Game/Sounds/MouseTrap.MouseTrap" "0, 0, 0" "0, 0, 0" 1.0 1.0 0.0 0 0 0)
          (bind _newtrack_0_2 (Timeline|Timeline_1 Play)
            (:Update
              (Transformation|SetRelativeRotation (Variables|Default|GetPivot) (Math|Rotator|Lerp(Rotator) (Variables|Default|GetStartPos) (Variables|Default|GetEndPos) _newtrack_0_2) false false)
              (Utilities|FlowControl|DoOnce false
                (:Completed
                  (Components|DestroyComponent (Variables|Default|GetBox)))))))))))

(fn ConstructionScript)